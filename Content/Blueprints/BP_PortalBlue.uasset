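; Blue portal actor that teleports the player through the portal manager when they enter it.
; On BeginPlay it looks up the human sprite character and the portal manager by class.
; On overlap, a dot product of its forward vector and the offset to the player limits triggering to the player on its back side, then it clears the manager's ToBlue flag and calls TeleportPlayer.
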(event `self.ReceiveBeginPlay`
  (bind _returnvalue (`GameplayStatics.GetActorOfClass` "/Game/Blueprints/BP_HumanSpriteCharacter.BP_HumanSpriteCharacter_C"))
  (bind _returnvalue_2 (`GameplayStatics.GetActorOfClass` "/Game/Blueprints/BP_PortalManager.BP_PortalManager_C")))

(event `self.ReceiveActorBeginOverlap`
  (params (OtherActor :type "Actor Object Reference"))
  (if (and (== (stale `self.ReceiveBeginPlay` _returnvalue) OtherActor) (< (`KismetMathLibrary.Dot_VectorVector` (`self.GetActorForwardVector`) (- (`self.K2_GetActorLocation` OtherActor) (`self.K2_GetActorLocation`))) 0.0))
    (set `/Game/Blueprints/BP_PortalManager.ToBlue?` false (stale `self.ReceiveBeginPlay` _returnvalue_2))
    (`/Game/Blueprints/BP_PortalManager.TeleportPlayer` (stale `self.ReceiveBeginPlay` _returnvalue_2))))

(fn `UserConstructionScript`)