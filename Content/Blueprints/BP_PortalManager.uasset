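; Portal manager that spawns blue and orange portals and teleports the player or physics objects between them, with ToBlue picking the destination.
; Tick spawns a portal at each unspawned BP_PortalSpawnPoint.
; TeleportObject cancels velocity by impulse, then re-adds it rotated about Y by the signed angle between portal forward vectors.
; TeleportPlayer moves the capsule but only prints the rotated velocity, as the node applying it is disconnected.
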(event `self.ReceiveBeginPlay`
  (bind _returnvalue (`GameplayStatics.GetActorOfClass` "/Game/Blueprints/BP_HumanSpriteCharacter.BP_HumanSpriteCharacter_C"))
  (set `self.Player` _returnvalue))

(event `TeleportPlayer`
  (bind _toblue_ (`self.ToBlue?`))
  (bind _capsulecomponent (`Character.CapsuleComponent` (`self.Player`)))
  (bind _returnvalue (`SceneComponent.GetForwardVector` (`PaperFlipbookActor.RenderComponent` (`self.BluePortal`))))
  (bind _returnvalue_2 (`SceneComponent.GetForwardVector` (`PaperFlipbookActor.RenderComponent` (`self.OrangePortal`))))
  (`KismetSystemLibrary.PrintString` (`KismetStringLibrary.BuildString_Bool` "Teleport Player" "ToBlue?=" _toblue_ "."))
  (`SceneComponent.K2_SetWorldLocation` _capsulecomponent (select `bool` _toblue_ :`false` (`self.K2_GetActorLocation` (`self.OrangePortal`)) :`true` (`self.K2_GetActorLocation` (`self.BluePortal`))) false true)
  (bind _output_get (set `self.OriginalVelocity` (`SceneComponent.GetComponentVelocity` _capsulecomponent)))
  (`KismetSystemLibrary.PrintString` "Hello")
  (`KismetSystemLibrary.PrintString` (`KismetStringLibrary.BuildString_Vector` "After Rotation Velocity = " "" (`KismetMathLibrary.RotateAngleAxis` _output_get (* (* (`KismetMathLibrary.DegAcos` (/ (`KismetMathLibrary.Dot_VectorVector` _returnvalue _returnvalue_2) (* (`KismetMathLibrary.VSize` _returnvalue) (`KismetMathLibrary.VSize` _returnvalue_2)))) (select `bool` (< (`KismetMathLibrary.Dot_VectorVector` (`KismetMathLibrary.Cross_VectorVector` _returnvalue _returnvalue_2) (0.0 1.0 0.0)) 0.0) :`false` 1 :`true` -1)) (select `bool` (`self.ToBlue?`) :`false` -1.0 :`true` 1.0)) (0.0 1.0 0.0)))))

(event `self.ReceiveTick`
  (params (DeltaSeconds :type "Float (single-precision)"))
  (bind _outactors (`GameplayStatics.GetAllActorsOfClass` "/Game/Blueprints/BP_PortalSpawnPoint.BP_PortalSpawnPoint_C"))
  (for _array_element _outactors
    (if (not (`/Game/Blueprints/BP_PortalSpawnPoint.HasSpawned?` _array_element))
      (`self.SpawnPortal`))))

(event `SpawnPortal`
  (if (`/Game/Blueprints/BP_PortalSpawnPoint.IsBlue?` (stale `self.ReceiveTick` _array_element))
    (bind _returnvalue (`self.GetTransform` (stale `self.ReceiveTick` _array_element)))
    (bind _returnvalue_2 (`|SpawnActorFromClass` "/Game/Blueprints/BP_PortalBlue.BP_PortalBlue_C" _returnvalue "Undefined" "MultiplyWithRoot" null null))
    (set `self.BluePortal` _returnvalue_2)
    (else
      (bind _returnvalue_3 (`|SpawnActorFromClass` "/Game/Blueprints/BP_PortalOrange.BP_PortalOrange_C" _returnvalue "Undefined" "MultiplyWithRoot" null null))
      (set `self.OrangePortal` _returnvalue_3)))
  (set `/Game/Blueprints/BP_PortalSpawnPoint.HasSpawned?` true (stale `self.ReceiveTick` _array_element)))

(fn `GetAngleBetwixtPortals`
  (returns (Angle :type "Float (double-precision)"))
  (bind _returnvalue (`SceneComponent.GetForwardVector` (`PaperFlipbookActor.RenderComponent` (`self.BluePortal`))))
  (bind _returnvalue_2 (`SceneComponent.GetForwardVector` (`PaperFlipbookActor.RenderComponent` (`self.OrangePortal`))))
  (return (* (* (`KismetMathLibrary.DegAcos` (/ (`KismetMathLibrary.Dot_VectorVector` _returnvalue _returnvalue_2) (* (`KismetMathLibrary.VSize` _returnvalue) (`KismetMathLibrary.VSize` _returnvalue_2)))) (select `bool` (< (`KismetMathLibrary.Dot_VectorVector` (`KismetMathLibrary.Cross_VectorVector` _returnvalue _returnvalue_2) (0.0 1.0 0.0)) 0.0) :`false` 1 :`true` -1)) (select `bool` (`self.ToBlue?`) :`false` -1.0 :`true` 1.0))))

(fn `TeleportObject`
  (params (`Actor Ref` :type "PrimitiveComponent Object Reference (by ref)"))
  (`SceneComponent.K2_SetWorldLocation` `Actor Ref` (select `bool` (`self.ToBlue?`) :`false` (`self.K2_GetActorLocation` (`self.OrangePortal`)) :`true` (`self.K2_GetActorLocation` (`self.BluePortal`))) false true) ; Update the location.
  (bind _returnvalue (`PrimitiveComponent.GetPhysicsLinearVelocity` `Actor Ref` "None")) ; Calculate force to cancel out object's current motion.
  (`PrimitiveComponent.AddImpulse` `Actor Ref` (* _returnvalue -1) "None" true) ; Add an instanteneous force to cancel out\nthe object's movement.
  (bind _angle (`self.GetAngleBetwixtPortals`))
  (`PrimitiveComponent.AddImpulse` `Actor Ref` (`KismetMathLibrary.RotateAngleAxis` _returnvalue _angle (0.0 1.0 0.0)) "None" true) ; Rotate the original velocity and \nadd it back to the object.
)

(fn `UserConstructionScript`)